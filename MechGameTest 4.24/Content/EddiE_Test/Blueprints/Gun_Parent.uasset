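; Base gun actor, meant to run as a child actor of a TankControls tank, that fires railgun projectiles.
; BeginFiring and StopFiring only toggle an IsFiring flag; nothing here reads it or calls FireBullet.
; FireBullet spawns a Railgun_Projectile at the barrel reference point using the tank body's rotation, overrides its initial and max speed with BulletSpeed, and decrements ammo without checking it.
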(event Custom|BeginFiring
  (Variables|Default|SetIsFiring true))

(event Custom|StopFiring
  (Variables|Default|SetIsFiring false))

(event EventBeginPlay)

(event Collision|EventActorBeginOverlap
  (params (OtherActor :type Actor%20Object%20Reference)))

(event EventTick
  (params (DeltaSeconds :type Float%20%28single-precision%29)))

(fn ConstructionScript)

(fn FireBullet
  (bind _bulletspeed (Variables|Default|GetBulletSpeed))
  (bind _astank_controls (Utilities|Casting|CastToTankControls (Actor|GetParentActor)))
  (bind _returnvalue (Game|SpawnActorfromClass "/Game/FirstPersonBP/Blueprints/Railgun_Projectile.Railgun_Projectile_C" (Math|Transform|MakeTransform (Transformation|GetWorldLocation (Variables|Default|GetBarrel_refpoint)) (Transformation|GetWorldRotation (Variables|/Game/FirstPersonBP/Blueprints/TankControls.TankControls_C|GetBody1 _astank_controls)) "1,1,1") "Undefined" 0 0))
  (Variables|/Script/Engine.ProjectileMovementComponent|SetInitialSpeed (Variables|/Game/FirstPersonBP/Blueprints/Railgun_Projectile.Railgun_Projectile_C|GetProjectileMovement _returnvalue) _bulletspeed)
  (Variables|/Script/Engine.ProjectileMovementComponent|SetMaxSpeed (Variables|/Game/FirstPersonBP/Blueprints/Railgun_Projectile.Railgun_Projectile_C|GetProjectileMovement _returnvalue) _bulletspeed)
  (Math|Integer|DecrementInt (Variables|Default|GetAmmoCurrent)))