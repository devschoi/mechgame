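; Railgun weapon Blueprint that charges while firing is held and releases a shot whose speed scales with the charge.
; A timeline paced by ChargeTime drives CurrentCharge, automatically releasing at full charge.
; Stopping fires only above a minimum charge, then reverses the timeline at normal rate, blocking recharging until it drains.
; FireBullet temporarily scales BulletSpeed around the parent call, then restores a hardcoded default.
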(event EventBeginFiring
  (|CallParentFunction)
  (if (and (not (Variables|Default|GetIsCharging)) (<= (Variables|Default|GetCurrentCharge) 0.2))
    (Variables|Default|SetIsCharging true)
    (Components|Timeline|SetPlayRate (Variables|Default|GetCharge_Weapon) (/ 1.0 (Variables|Default|GetChargeTime)))
    (bind _weaponcharge (Timeline|Charge_Weapon Play)
      (:Update
        (bind _output_get (Variables|Default|SetCurrentCharge (Math|Float|Clamp(Float) _weaponcharge)))
        (if (>= _output_get 1.0)
          (CallFunction|StopFiring))))))

(event EventStopFiring
  (|CallParentFunction)
  (if (and (Variables|Default|GetIsCharging) (>= (Variables|Default|GetCurrentCharge) 0.2))
    (CallFunction|FireBullet))
  (Variables|Default|SetIsCharging false)
  (Components|Timeline|SetPlayRate (Variables|Default|GetCharge_Weapon) 1.0)
  (bind _weaponcharge (Timeline|Charge_Weapon Reverse)
    (:Update
      (bind _output_get (Variables|Default|SetCurrentCharge (Math|Float|Clamp(Float) _weaponcharge)))
      (if (>= _output_get 1.0)
        (CallFunction|StopFiring)))))

(fn ConstructionScript
  (|CallParentFunction))

(fn FireBullet
  (Variables|Default|SetBulletSpeed (* (Variables|Default|GetBulletSpeed) (Variables|Default|GetCurrentCharge)))
  (|CallParentFunction)
  (Variables|Default|SetBulletSpeed 3e+03))