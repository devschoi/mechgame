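; FullyAuto_Gun is a gun Blueprint that fires automatically for as long as firing is active.
; BeginFiring calls the parent, fires one bullet immediately, then starts a looping timer that calls FireBullet by name at the FireRate interval.
; StopFiring calls the parent and clears the stored GunTimer handle to end the loop.
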(event EventBeginFiring
  (|CallParentFunction)
  (CallFunction|FireBullet)
  (bind _returnvalue (Utilities|Time|SetTimerbyFunctionName 0 "FireBullet" (Variables|Default|GetFireRate) true))
  (Variables|Default|SetGunTimer _returnvalue))

(event EventStopFiring
  (|CallParentFunction)
  (Utilities|Time|ClearandInvalidateTimerbyHandle (Variables|Default|GetGunTimer)))

(fn ConstructionScript
  (|CallParentFunction))